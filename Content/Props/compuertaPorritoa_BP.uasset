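; Puzzle gate that opens its two doors once three rotatable cylinders each face their target direction.
; Tick compares each cylinder's yaw to an exact float value, showing its beam (Haz) and disabling its input when it matches.
; When all three match, a DoOnce deactivates two security cameras, then after a delay plays a door sound and a timeline slides the doors, found through GetActorOfClass on its own class.
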(event `self.ReceiveTick`
  (params (DeltaSeconds :type "Float (single-precision)"))
  (bind _cilindro1 (`self.Cilindro1`))
  (bind _cilindro2 (`self.Cilindro2`))
  (bind _cilindro3 (`self.Cilindro3`))
  (bind (_returnvalue_roll _returnvalue_pitch _returnvalue_yaw) (`KismetMathLibrary.BreakRotator` (`self.K2_GetActorRotation` (`self.Cilindro3`))))
  (bind (_returnvalue_roll_2 _returnvalue_pitch_2 _returnvalue_yaw_2) (`KismetMathLibrary.BreakRotator` (`self.K2_GetActorRotation` (`self.Cilindro1`))))
  (bind (_returnvalue_roll_3 _returnvalue_pitch_3 _returnvalue_yaw_3) (`KismetMathLibrary.BreakRotator` (`self.K2_GetActorRotation` (`self.Cilindro2`))))
  (bind _returnvalue (== _returnvalue_yaw 89.999985))
  (bind _returnvalue_2 (== _returnvalue_yaw_3 179.999954))
  (bind _returnvalue_3 (== _returnvalue_yaw_2 -90.000053))
  (`|ExecutionSequence`
    (:`then_0`
      (if (and _returnvalue_3 _returnvalue_2 _returnvalue)
        (`/Engine/EditorBlueprintResources/StandardMacros.DoOnce` false
          (:`Completed`
            (`/Game/ThirdPersonBP/Blueprints/SecCamera_BP_MOV.DeactivateCamera` (`self.SecCamera`))
            (`/Game/ThirdPersonBP/Blueprints/SecCamera_BP_MOV.DeactivateCamera` (`self.SecCamera_0`))
            (bind _returnvalue_4 (`GameplayStatics.GetActorOfClass` "compuertaPorritoa_BP_C"))
            (`KismetSystemLibrary.Delay` 1.5)
            (`GameplayStatics.PlaySoundAtLocation` "/Game/Audio/Door_SoundCUe.Door_SoundCUe" (0.0 0.0 0.0) (struct) 1.0 1.0 0.0 null null null)
            (bind (_direction _door1 _door2) (`Timeline|Timeline_0`)
              (:`Update`
                (`|ExecutionSequence`
                  (:`then_0`
                    (`SceneComponent.K2_SetRelativeLocation` (`/Game/Props/compuertaPorritoa_BP.Puerta1` _returnvalue_4) (`KismetMathLibrary.MakeVector` _door1 0.0 190.0) false false))
                  (:`then_1`
                    (`SceneComponent.K2_SetRelativeLocation` (`/Game/Props/compuertaPorritoa_BP.puerta2` _returnvalue_4) (`KismetMathLibrary.MakeVector` _door2 0.0 190.0) false false)))))))))
    (:`then_1`
      (if _returnvalue_3
        (`SceneComponent.SetVisibility` (`/Game/CilindroPuzzle_BP.Haz` _cilindro1) true false)
        (`self.DisableInput` _cilindro1 null)))
    (:`then_2`
      (if _returnvalue_2
        (`SceneComponent.SetVisibility` (`/Game/CilindroPuzzle_BP_2.Haz` _cilindro2) true false)
        (`self.DisableInput` _cilindro2 null)))
    (:`then_3`
      (if _returnvalue
        (`SceneComponent.SetVisibility` (`/Game/CilindroPuzzle_BP_3.Haz` _cilindro3) true false)
        (`self.DisableInput` _cilindro3 null)))))

(fn `UserConstructionScript`)