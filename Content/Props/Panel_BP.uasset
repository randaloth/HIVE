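; Interactable panel prop that loads level "Porritoa" when the player holds Interact nearby, provided Palanca's Interaction flag is set; otherwise it plays a sound.
; Box overlap toggles the hold prompt, input and progress-bar widget, using a Gate and mutually resetting DoOnce nodes.
; Pressing plays the character animation, starts a retriggerable delay that checks IsHeld, and polls a timer to fill the bar.
; Separate events switch the panel's emissive material on or off.
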(event `ActivateEmissive`
  ;[1 1 1] Activate Emissive
  (bind _returnvalue (`PrimitiveComponent.CreateDynamicMaterialInstance` (`self.PanelHigh`) 0 "/Game/Props/Textures_Panel/Panel_Mat.Panel_Mat" "None"))
  (`MaterialInstanceDynamic.SetScalarParameterValue` _returnvalue "Emissive" 1.0))

(event `ResetPanel`
  (bind _returnvalue (`PrimitiveComponent.CreateDynamicMaterialInstance` (`self.PanelHigh`) 0 "/Game/Props/Textures_Panel/Panel_Mat.Panel_Mat" "None"))
  (`MaterialInstanceDynamic.SetScalarParameterValue` _returnvalue "Emissive" 0.0)
  (set `self.IsHeld?` false))

(event `InputAction|Interact`
  (params (Key :type "Key Structure"))
  (:`Pressed`
    (set `self.IsHeld?` true)
    (if (`/Game/Props/palanca_BP.Interaction` (`self.palanca`))
      (`/Engine/EditorBlueprintResources/StandardMacros.Gate` true :!label _label
        (:`Exit`
          (bind _asthird_person_character (cast `/Game/ThirdPersonBP/Blueprints/ThirdPersonCharacter` (`GameplayStatics.GetPlayerCharacter` 0)))
          (`/Game/ThirdPersonBP/Blueprints/ThirdPersonCharacter.InteractAnim` _asthird_person_character)
          (`|ExecutionSequence`
            (:`then_0`
              (`KismetSystemLibrary.RetriggerableDelay` (`self.MaxHoldTime`))
              (if (`self.IsHeld?`)
                (`GameplayStatics.OpenLevel` "Porritoa")))
            (:`then_1`
              (`self.Timer`)
              (`self.Update Timer`)))))
      (else
        ;[1 1 1] AUDIO ALBA
        (`GameplayStatics.PlaySoundAtLocation` null (0.0 0.0 0.0) (struct) 1.0 1.0 0.0 null null null))))
  (:`Released`
    (set `self.IsHeld?` false)))

(event `ResetStart`
  (goto _label_2 :!via `Reset`))

(event `self.Box.OnComponentBeginOverlap`
  (params (OverlappedComponent :type "PrimitiveComponent Object Reference") (OtherActor :type "Actor Object Reference") (OtherComp :type "PrimitiveComponent Object Reference") (OtherBodyIndex :type Integer) (bFromSweep :type Boolean) (SweepResult :type "HitResult Structure (by ref)"))
  (`SceneComponent.SetVisibility` (`self.HoldE`) true false)
  (`/Engine/EditorBlueprintResources/StandardMacros.DoOnce` false :!label _label_2
    (:`Completed`
      (cast `/Game/ThirdPersonBP/Blueprints/ThirdPersonCharacter` OtherActor)
      (`self.EnableInput` (`GameplayStatics.GetPlayerController` 0))
      (bind _returnvalue (`|CreateWidget` "/Game/Props/Progres_Bar.Progres_Bar_C"))
      (bind _output_get (set `self.Widget Ref` _returnvalue))
      (`UserWidget.AddToViewport` _output_get 0)
      (set `/Game/Props/Progres_Bar.MaxTimeHeld` (`self.MaxHoldTime`) _output_get)
      (`|ExecutionSequence`
        (:`then_0`
          (goto _label :!via `Open`))
        (:`then_1`
          (`self.ResetEnd`))))))

(event `self.Box.OnComponentEndOverlap`
  (params (OverlappedComponent :type "PrimitiveComponent Object Reference") (OtherActor :type "Actor Object Reference") (OtherComp :type "PrimitiveComponent Object Reference") (OtherBodyIndex :type Integer))
  (`SceneComponent.SetVisibility` (`self.HoldE`) false false)
  (`/Engine/EditorBlueprintResources/StandardMacros.DoOnce` false :!label _label_3
    (:`Completed`
      (cast `/Game/ThirdPersonBP/Blueprints/ThirdPersonCharacter` OtherActor)
      (`self.DisableInput` (`GameplayStatics.GetPlayerController` 0))
      (`Widget.RemoveFromParent` (stale `self.Box.OnComponentBeginOverlap` _returnvalue))
      (`|ExecutionSequence`
        (:`then_0`
          (goto _label :!via `Close`))
        (:`then_1`
          (`self.ResetStart`))))))

(event `Stop Timer`
  ;[1 1 1] Timer
  (`KismetSystemLibrary.K2_PauseTimerHandle` (stale `Timer` _returnvalue)))

(event `Timer`
  ;[1 1 1] Timer
  (bind _returnvalue (`KismetSystemLibrary.K2_SetTimerDelegate` (delegate `Timer`) (`self.MaxHoldTime`))))

(event `ResetEnd`
  (goto _label_3 :!via `Reset`))

(event `Update Timer`
  (bind _widget_ref (`self.Widget Ref`))
  ;[1 1 1] Timer
  (if (`self.IsHeld?`)
    (set `/Game/Props/Progres_Bar.TimeHeld` (`KismetSystemLibrary.K2_GetTimerElapsedTimeHandle` (stale `Timer` _returnvalue)) _widget_ref)
    (`KismetSystemLibrary.Delay` 0.1)
    (`self.Update Timer`)
    (else
      (`self.Stop Timer`)
      (set `/Game/Props/Progres_Bar.TimeHeld` 0.0 _widget_ref))))

(fn `UserConstructionScript`)