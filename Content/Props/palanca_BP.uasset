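; Lever prop that the player activates with Interact while inside its Box, playing the character's interact animation, lighting its Panel and activating Fog.
; A Gate driven by box overlap filters the input, and a DoOnce limits it to one use.
; The first Trigger_palanca overlap starts a timeline moving a hint marker vertically, shown after a delay if the lever is still unused.
; ResetPalanca resets the panel and re-arms both DoOnces.
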(event `self.Trigger_palanca.OnActorBeginOverlap`
  (params (OverlappedActor :type "Actor Object Reference") (OtherActor :type "Actor Object Reference"))
  (`/Engine/EditorBlueprintResources/StandardMacros.DoOnce` false :!label _label
    (:`Completed`
      (`|ExecutionSequence`
        (:`then_0`
          (`KismetSystemLibrary.Delay` 10.0)
          (if (not (`self.Interaction`))
            (`SceneComponent.SetVisibility` (`self.Marcador`) true false)))
        (:`then_1`
          (bind (_direction _movement) (`Timeline|Timeline_0`)
            (:`Update`
              (`SceneComponent.K2_SetRelativeLocation` (`self.Marcador`) (`KismetMathLibrary.MakeVector` 19.0 0.0 (`KismetMathLibrary.Lerp` 110.0 140.0 _movement)) false false))))))))

(event `ResetPalanca`
  (set `self.Interaction` false)
  (`/Game/Props/Panel_BP.ResetPanel` (`self.Panel`))
  (`|ExecutionSequence`
    (:`then_0`
      (goto _label :!via `Reset`))
    (:`then_1`
      (goto _label_3 :!via `Reset`))))

(event `self.ReceiveBeginPlay`
  (`self.EnableInput` (`GameplayStatics.GetPlayerController` 0)))

(event `InputAction|Interact` :consume false
  (params (Key :type "Key Structure"))
  (:`Pressed`
    (`/Engine/EditorBlueprintResources/StandardMacros.Gate` true :!label _label_2
      (:`Exit`
        (`/Engine/EditorBlueprintResources/StandardMacros.DoOnce` false :!label _label_3
          (:`Completed`
            (bind _asthird_person_character (cast `/Game/ThirdPersonBP/Blueprints/ThirdPersonCharacter` (`GameplayStatics.GetPlayerCharacter` 0)))
            (`/Game/ThirdPersonBP/Blueprints/ThirdPersonCharacter.InteractAnim` _asthird_person_character)
            (set `self.Interaction` true)
            (`/Game/Props/Panel_BP.ActivateEmissive` (`self.Panel`))
            (`SceneComponent.SetVisibility` (`self.Marcador`) false false)
            (`/Game/Fog/Fog_BP.Activate` (`self.Fog`))))))))

(event `self.Box.OnComponentBeginOverlap`
  (params (OverlappedComponent :type "PrimitiveComponent Object Reference") (OtherActor :type "Actor Object Reference") (OtherComp :type "PrimitiveComponent Object Reference") (OtherBodyIndex :type Integer) (bFromSweep :type Boolean) (SweepResult :type "HitResult Structure (by ref)"))
  (cast `/Game/ThirdPersonBP/Blueprints/ThirdPersonCharacter` OtherActor)
  (goto _label_2 :!via `Open`))

(event `self.Box.OnComponentEndOverlap`
  (params (OverlappedComponent :type "PrimitiveComponent Object Reference") (OtherActor :type "Actor Object Reference") (OtherComp :type "PrimitiveComponent Object Reference") (OtherBodyIndex :type Integer))
  (cast `/Game/ThirdPersonBP/Blueprints/ThirdPersonCharacter` OtherActor)
  (goto _label_2 :!via `Close`))

(fn `UserConstructionScript`)