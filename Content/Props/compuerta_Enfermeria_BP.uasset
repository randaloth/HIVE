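; Infirmary sliding double door that shows a password widget (UI_CONTRASEÑA) and mouse cursor while the ThirdPersonCharacter is inside its trigger.
; Two cross-resetting DoOnce gates pair overlap begin and end, so a single widget is created on entry and removed on exit.
; Abrir_Puertas, not called here although the widget receives a door reference, destroys the trigger once, then after a delay plays a sound and slides both panels via Timeline.
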(event `self.Trigger_UI.OnComponentBeginOverlap`
  (params (OverlappedComponent :type "PrimitiveComponent Object Reference") (OtherActor :type "Actor Object Reference") (OtherComp :type "PrimitiveComponent Object Reference") (OtherBodyIndex :type Integer) (bFromSweep :type Boolean) (SweepResult :type "HitResult Structure (by ref)"))
  ;[1 1 1] UI
  (bind _asthird_person_character (cast `/Game/ThirdPersonBP/Blueprints/ThirdPersonCharacter` OtherActor))
  (`/Engine/EditorBlueprintResources/StandardMacros.IsValid` _asthird_person_character
    (:`Is Valid`
      (`/Engine/EditorBlueprintResources/StandardMacros.DoOnce` false :!label _label
        (:`Completed`
          (bind _returnvalue (`|CreateWidget` "/Game/Environment/HIVE_REBUILD/UI_CONTRASEÑA.UI_CONTRASEÑA_C"))
          (bind _output_get (set `self.UI` _returnvalue))
          (set `/Game/Environment/HIVE_REBUILD/UI_CONTRASEÑA.Puerta_Enfermeria` self _output_get)
          (`UserWidget.AddToViewport` _output_get 0)
          (set `PlayerController.bShowMouseCursor` true (`GameplayStatics.GetPlayerController` 0))
          (goto _label_2 :!via `Reset`))))))

(event `Abrir_Puertas`
  ;[1 1 1] Abrir Puertas
  (`/Engine/EditorBlueprintResources/StandardMacros.DoOnce` false
    (:`Completed`
      (`ActorComponent.K2_DestroyComponent` (`self.Trigger_UI`))
      (`KismetSystemLibrary.Delay` 1.5)
      (`GameplayStatics.PlaySoundAtLocation` "/Game/Audio/Door_SoundCUe.Door_SoundCUe" (`self.K2_GetActorLocation`) (struct) 1.0 1.0 0.0 null null null)
      (bind (_direction _door1 _door2) (`Timeline|Timeline_0`)
        (:`Update`
          (`|ExecutionSequence`
            (:`then_0`
              (`SceneComponent.K2_SetRelativeLocation` (`self.Puerta1`) (`KismetMathLibrary.MakeVector` _door1 0.0 190.0) false false))
            (:`then_1`
              (`SceneComponent.K2_SetRelativeLocation` (`self.puerta2`) (`KismetMathLibrary.MakeVector` _door2 0.0 190.0) false false))))))))

(event `self.Trigger_UI.OnComponentEndOverlap`
  (params (OverlappedComponent :type "PrimitiveComponent Object Reference") (OtherActor :type "Actor Object Reference") (OtherComp :type "PrimitiveComponent Object Reference") (OtherBodyIndex :type Integer))
  ;[1 1 1] UI
  (bind _asthird_person_character (cast `/Game/ThirdPersonBP/Blueprints/ThirdPersonCharacter` OtherActor))
  (`/Engine/EditorBlueprintResources/StandardMacros.IsValid` _asthird_person_character
    (:`Is Valid`
      (`/Engine/EditorBlueprintResources/StandardMacros.DoOnce` false :!label _label_2
        (:`Completed`
          (`Widget.RemoveFromParent` (`self.UI`))
          (set `PlayerController.bShowMouseCursor` false (`GameplayStatics.GetPlayerController` 0))
          (goto _label :!via `Reset`))))))

(fn `UserConstructionScript`)