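; Gate controller that opens the two-panel door of a Compuerta_BP actor once a Button_BP is pressed.
; Tick looks up the button by class every frame and polls its Pressed flag, with a DoOnce limiting the opening to one run.
; After a short delay it plays a door sound at the world origin, then a timeline slides the right and left panels along X at fixed height.
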(event `self.ReceiveTick`
  (params (DeltaSeconds :type "Float (single-precision)"))
  (bind _returnvalue (`GameplayStatics.GetActorOfClass` "/Game/ThirdPersonBP/Blueprints/Button_BP.Button_BP_C"))
  (if (`/Game/ThirdPersonBP/Blueprints/Button_BP.Pressed?` _returnvalue)
    (`/Engine/EditorBlueprintResources/StandardMacros.DoOnce` false
      (:`Completed`
        (bind _returnvalue_2 (`GameplayStatics.GetActorOfClass` "/Game/Props/compuerta_BP.compuerta_BP_C"))
        (`KismetSystemLibrary.Delay` 1.5)
        (`GameplayStatics.PlaySoundAtLocation` "/Game/Audio/Door_SoundCUe.Door_SoundCUe" (0.0 0.0 0.0) (struct) 1.0 1.0 0.0 null null null)
        (bind (_direction _door1 _door2) (`Timeline|Timeline_0`)
          (:`Update`
            (`|ExecutionSequence`
              (:`then_0`
                (`SceneComponent.K2_SetRelativeLocation` (`/Game/Props/compuerta_BP.Puerta_derecha` _returnvalue_2) (`KismetMathLibrary.MakeVector` _door1 0.0 190.0) false false))
              (:`then_1`
                (`SceneComponent.K2_SetRelativeLocation` (`/Game/Props/compuerta_BP.puerta_izquierda` _returnvalue_2) (`KismetMathLibrary.MakeVector` _door2 0.0 190.0) false false)))))))))

(fn `UserConstructionScript`)