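; Corridor alarm light Blueprint with a rotating spotlight and a trigger that sets off an alarm sound.
; A timeline started on BeginPlay drives the spotlight's yaw through a full turn.
; Any actor overlapping the trigger makes the light visible and, through a DoOnce, spawns a single 2D alarm loop.
; The Reset event hides the light, stops the alarm and re-arms the DoOnce.
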(event `self.ReceiveBeginPlay`
  (bind (_direction _rotacion) (`Timeline|Timeline_0`)
    (:`Update`
      (`SceneComponent.K2_SetRelativeRotation` (`self.SpotLight`) (`KismetMathLibrary.MakeRotator` 0.0 0.0 (`KismetMathLibrary.Lerp` 0.0 360.0 _rotacion)) false false))))

(event `self.Trigger.OnActorBeginOverlap`
  (params (OverlappedActor :type "Actor Object Reference") (OtherActor :type "Actor Object Reference"))
  (`SceneComponent.SetVisibility` (`self.SpotLight`) true true)
  (`/Engine/EditorBlueprintResources/StandardMacros.DoOnce` false :!label _label
    (:`Completed`
      (bind _returnvalue (`GameplayStatics.SpawnSound2D` "/Game/Audio/alarmloop_Cue.alarmloop_Cue" 1.0 1.0 0.0 null))
      (set `self.alarm` _returnvalue))))

(event `Reset`
  (`SceneComponent.SetVisibility` (`self.SpotLight`) false true)
  (`AudioComponent.Stop` (`self.alarm`))
  (goto _label :!via `Reset`))

(fn `UserConstructionScript`)