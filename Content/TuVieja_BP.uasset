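; Interactable actor whose Cylinder rotates 90 degrees in yaw when the player presses Interact nearby.
; Capsule overlaps with the ThirdPersonCharacter open and close a Gate that filters the input.
; Each accepted press captures the current relative yaw and restarts the Rotation timeline, which lerps toward a target a quarter turn further in a fixed positive direction.
; During updates, a world yaw of exactly 360 resets the stored start rotation to zero.
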(event `InputAction|Interact`
  (params (Key :type "Key Structure"))
  (bind (_returnvalue_roll _returnvalue_pitch _returnvalue_yaw) (`KismetMathLibrary.BreakRotator` (`SceneComponent.K2_GetComponentRotation` (`self.Cylinder`))))
  (bind (_relativerotation_roll _relativerotation_pitch _relativerotation_yaw) (`KismetMathLibrary.BreakRotator` (`SceneComponent.RelativeRotation` (`self.Cylinder`))))
  (:`Pressed`
    (`/Engine/EditorBlueprintResources/StandardMacros.Gate` true :!label _label
      (:`Exit`
        (`KismetSystemLibrary.PrintString` "rota")
        (set `self.Current Rotation` _relativerotation_yaw)
        (set `self.Target Rotation` (+ (* (select `bool` true :`false` -1.0 :`true` 1.0 :!type "Float (single-precision)") 90.0) (`self.Current Rotation`)))
        (bind (_direction _rotacio) (`Timeline|rotation` :!via `PlayFromStart`)
          (:`Update`
            (`SceneComponent.K2_SetRelativeRotation` (`self.Cylinder`) (`KismetMathLibrary.MakeRotator` 0.0 0.0 (`KismetMathLibrary.Lerp` (`self.Current Rotation`) (`self.Target Rotation`) _rotacio)) false false)
            (if (== _returnvalue_yaw 360.0)
              (set `self.Current Rotation` 0.0))))))))

(event `self.Capsule.OnComponentBeginOverlap`
  (params (OverlappedComponent :type "PrimitiveComponent Object Reference") (OtherActor :type "Actor Object Reference") (OtherComp :type "PrimitiveComponent Object Reference") (OtherBodyIndex :type Integer) (bFromSweep :type Boolean) (SweepResult :type "HitResult Structure (by ref)"))
  (cast `/Game/ThirdPersonBP/Blueprints/ThirdPersonCharacter` OtherActor)
  (goto _label :!via `Open`))

(event `self.Capsule.OnComponentEndOverlap`
  (params (OverlappedComponent :type "PrimitiveComponent Object Reference") (OtherActor :type "Actor Object Reference") (OtherComp :type "PrimitiveComponent Object Reference") (OtherBodyIndex :type Integer))
  (cast `/Game/ThirdPersonBP/Blueprints/ThirdPersonCharacter` OtherActor)
  (goto _label :!via `Close`))

(fn `UserConstructionScript`)