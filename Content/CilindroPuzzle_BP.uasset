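; Rotatable puzzle cylinder actor that turns 90 degrees in yaw when the player presses Interact nearby.
; Capsule overlap with ThirdPersonCharacter opens and closes a Gate on that input.
; The Rotation timeline lerps actor yaw to the target, with a DoOnce reset on finish, though presses mid-turn still overwrite the lerp's start yaw.
; Debug prints run on interaction and every Tick; disconnected nodes hold unused rotation and wrap logic.
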(event `InputAction|Interact` :consume false :overrideparent false
  (params (Key :type "Key Structure"))
  (bind (_returnvalue_roll _returnvalue_pitch _returnvalue_yaw) (`KismetMathLibrary.BreakRotator` (`self.K2_GetActorRotation`)))
  (:`Pressed`
    (`/Engine/EditorBlueprintResources/StandardMacros.Gate` true :!label _label
      (:`Exit`
        (`KismetSystemLibrary.PrintString` "rota")
        (set `self.Current Rotation` _returnvalue_yaw)
        (`/Engine/EditorBlueprintResources/StandardMacros.DoOnce` false :!label _label_2
          (:`Completed`
            (set `self.Target Rotation` (+ (`self.Current Rotation`) 90.0))
            (bind (_direction _rotacio) (`Timeline|rotation` :!via `PlayFromStart`)
              (:`Update`
                (`self.K2_SetActorRotation` (`KismetMathLibrary.MakeRotator` 0.0 0.0 (`KismetMathLibrary.Lerp` (`self.Current Rotation`) (`self.Target Rotation`) _rotacio))))
              (:`Finished`
                (goto _label_2 :!via `Reset`)))))))))

(event `self.Capsule.OnComponentBeginOverlap`
  (params (OverlappedComponent :type "PrimitiveComponent Object Reference") (OtherActor :type "Actor Object Reference") (OtherComp :type "PrimitiveComponent Object Reference") (OtherBodyIndex :type Integer) (bFromSweep :type Boolean) (SweepResult :type "HitResult Structure (by ref)"))
  (cast `/Game/ThirdPersonBP/Blueprints/ThirdPersonCharacter` OtherActor)
  (goto _label :!via `Open`))

(event `self.Capsule.OnComponentEndOverlap`
  (params (OverlappedComponent :type "PrimitiveComponent Object Reference") (OtherActor :type "Actor Object Reference") (OtherComp :type "PrimitiveComponent Object Reference") (OtherBodyIndex :type Integer))
  (cast `/Game/ThirdPersonBP/Blueprints/ThirdPersonCharacter` OtherActor)
  (goto _label :!via `Close`))

(event `self.ReceiveTick`
  (params (DeltaSeconds :type "Float (single-precision)"))
  (bind (_returnvalue_roll _returnvalue_pitch _returnvalue_yaw) (`KismetMathLibrary.BreakRotator` (`self.K2_GetActorRotation`)))
  (`KismetSystemLibrary.PrintString` (`KismetStringLibrary.Conv_DoubleToString` _returnvalue_yaw)))

(fn `UserConstructionScript`)